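; Falling_Point_BP is a placeable trigger point that registers itself with the player character when touched.
; On sphere overlap, it casts the other actor to Player_BP and passes itself to AddFallingPoints if it is not already in that player's FallingPoints array.
; The construction script sizes the trigger sphere from the SphereRadius variable.
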(event `self.Sphere.OnComponentBeginOverlap`
  (params (OverlappedComponent :type "PrimitiveComponent Object Reference") (OtherActor :type "Actor Object Reference") (OtherComp :type "PrimitiveComponent Object Reference") (OtherBodyIndex :type Integer) (bFromSweep :type Boolean) (SweepResult :type "HitResult Structure (by ref)"))
  (bind _asplayer_bp (cast `/Game/Platformer/Blueprints/Player/Player_BP` OtherActor))
  (if (== (`KismetArrayLibrary.Array_Find` (`/Game/Platformer/Blueprints/Player/Player_BP.Falling Points` _asplayer_bp) self) -1)
    (`/Game/Platformer/Blueprints/Player/Player_BP.Add FallingPoints` _asplayer_bp self)))

(fn `UserConstructionScript`
  (`SphereComponent.SetSphereRadius` (`self.Sphere`) (`self.Sphere radius`) true))