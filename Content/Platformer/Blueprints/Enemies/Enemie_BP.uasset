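; Enemy character for a platformer that follows the player, fires fireballs and knocks back players who get too close.
; Tick distance checks drive movement, smoothed turning, attack start and cooldown-limited knockback; trigger overlaps also start attacks.
; LaunchAttack messages the AnimInstance and re-arms on a random timer, while separate events handle charge Niagara effects and spawn player-aimed projectiles.
; Hits decrement life and briefly suppress knockback; death disables capsule collision and grants the player a heal.
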(event `self.Attack_trigger.OnComponentBeginOverlap`
  (params (OverlappedComponent :type "PrimitiveComponent Object Reference") (OtherActor :type "Actor Object Reference") (OtherComp :type "PrimitiveComponent Object Reference") (OtherBodyIndex :type Integer) (bFromSweep :type Boolean) (SweepResult :type "HitResult Structure (by ref)"))
  (cast `/Game/Platformer/Blueprints/Player/Player_BP` OtherActor)
  (set `self.Attack_trigger_activate` true)
  (set `self.Can follow` false)
  (`self.Launch Attack`))

(event `self.Attack_trigger.OnComponentEndOverlap`
  (params (OverlappedComponent :type "PrimitiveComponent Object Reference") (OtherActor :type "Actor Object Reference") (OtherComp :type "PrimitiveComponent Object Reference") (OtherBodyIndex :type Integer))
  (cast `/Game/Platformer/Blueprints/Player/Player_BP` OtherActor)
  (set `self.Attack_trigger_activate` false)
  (set `self.Can follow` true))

(event `self.Follow_trigger.OnComponentEndOverlap`
  (params (OverlappedComponent :type "PrimitiveComponent Object Reference") (OtherActor :type "Actor Object Reference") (OtherComp :type "PrimitiveComponent Object Reference") (OtherBodyIndex :type Integer))
  (cast `/Game/Platformer/Blueprints/Player/Player_BP` OtherActor)
  (set `self.Follow_trigger_activate` false))

(event `self.Follow_trigger.OnComponentBeginOverlap`
  (params (OverlappedComponent :type "PrimitiveComponent Object Reference") (OtherActor :type "Actor Object Reference") (OtherComp :type "PrimitiveComponent Object Reference") (OtherBodyIndex :type Integer) (bFromSweep :type Boolean) (SweepResult :type "HitResult Structure (by ref)"))
  (cast `/Game/Platformer/Blueprints/Player/Player_BP` OtherActor)
  (set `self.Follow_trigger_activate` true))

(event `self.ReceiveBeginPlay`
  (bind _outactors (`GameplayStatics.GetAllActorsOfClass` "/Game/Platformer/Blueprints/Player/Player_BP.Player_BP_C"))
  (set `self.Player_ref` (`|GetArrayItem` _outactors))
  (bind _aslife_bar_w (cast `/Game/Platformer/Widgets/Life_Bar_W` (`WidgetComponent.GetWidget` (`self.Life Bar`))))
  (set `/Game/Platformer/Widgets/Life_Bar_W.Enemie` self _aslife_bar_w)
  (set `/Game/Platformer/Widgets/Life_Bar_W.Init life` (`self.Life`) _aslife_bar_w))

(event `self.ReceiveTick`
  (params (DeltaSeconds :type "Float (single-precision)"))
  (bind _returnvalue (`self.K2_GetActorLocation`))
  (bind (_returnvalue_roll _returnvalue_pitch _returnvalue_yaw) (`KismetMathLibrary.BreakRotator` (`self.K2_GetActorRotation`)))
  (bind _returnvalue_2 (`self.GetController`))
  (bind _returnvalue_3 (`self.K2_GetActorLocation` (`self.Player_ref`)))
  (bind (_returnvalue_roll_2 _returnvalue_pitch_2 _returnvalue_yaw_2) (`KismetMathLibrary.BreakRotator` (`KismetMathLibrary.FindLookAtRotation` _returnvalue _returnvalue_3)))
  (bind _returnvalue_4 (`KismetMathLibrary.Vector_Distance` _returnvalue_3 _returnvalue))
  (`/Engine/EditorBlueprintResources/StandardMacros.IsValid` _returnvalue_2
    (:`Is Valid`
      (`|ExecutionSequence`
        (:`then_0`
          (if (and (< _returnvalue_4 (`self.Follow Distance`)) (not (`self.Dead`)))
            (if (> _returnvalue_4 (`self.Follow Min Dist`))
              (`AIBlueprintHelperLibrary.SimpleMoveToLocation` _returnvalue_2 _returnvalue_3)
              (`self.K2_SetActorRotation` (`KismetMathLibrary.MakeRotator` _returnvalue_roll _returnvalue_pitch (`KismetMathLibrary.FInterpTo` _returnvalue_yaw _returnvalue_yaw_2 DeltaSeconds 5.0)) :!label _label)
              (else
                (`|ExecutionSequence`
                  (:`then_0`
                    (goto _label))
                  (:`then_1`
                    (`Controller.StopMovement` _returnvalue_2 :!label _label_2)))))
            (else
              (goto _label_2))))
        (:`then_1`
          (if (and (< _returnvalue_4 (`self.Attack Distance`)) (not (`self.Dead`)))
            (`/Engine/EditorBlueprintResources/StandardMacros.DoOnce` false :!label _label_3
              (:`Completed`
                (`self.Launch Attack`)))
            (else
              (goto _label_3 :!via `Reset`))))
        (:`then_2`
          (`self.KnockPlayer`))))))

(event `Take Damage`
  (bind _returnvalue (`SkeletalMeshComponent.GetAnimInstance` (`self.Mesh`)))
  (if (not (`self.Dead`))
    (`/Engine/EditorBlueprintResources/StandardMacros.DecrementInt` (`self.Life`)
      (:`  `
        (if (> (`self.Life`) 0)
          (message `/Game/Platformer/Blueprints/Player/Animations/Player_Anim_BP.Hit` _returnvalue)
          (set `self.Can Knock` false)
          (`KismetSystemLibrary.Delay` 2.0)
          (set `self.Can Knock` true)
          (else
            (message `/Game/Platformer/Blueprints/Player/Animations/Player_Anim_BP.Die` _returnvalue)
            (set `self.Dead` true)
            (`PrimitiveComponent.SetCollisionEnabled` (`self.CapsuleComponent`) "NoCollision")
            (`/Engine/EditorBlueprintResources/StandardMacros.IncrementInt` (`/Game/Platformer/Blueprints/Player/Player_BP.Number of heal` (`self.Player_ref`)))))))))

(event `Launch Attack`
  (bind (_freq_attack_x _freq_attack_y) (`KismetMathLibrary.BreakVector2D` (`self.Freq Attack`)))
  (if (and (not (`self.Dead`)) (not (`/Game/Platformer/Blueprints/Player/Player_BP.Dead` (`self.Player_ref`))))
    (message `/Game/Platformer/Blueprints/Player/Animations/Player_Anim_BP.Attack` (`SkeletalMeshComponent.GetAnimInstance` (`self.Mesh`)))
    (`KismetSystemLibrary.K2_SetTimerDelegate` (delegate `Launch Attack`) (`KismetMathLibrary.RandomFloatInRange` _freq_attack_x _freq_attack_y))
    (set `self.Can Knock` false)
    (`KismetSystemLibrary.Delay` 1.0)
    (set `self.Can Knock` true)))

(event `/Game/Platformer/Blueprints/Player/Animations/Player_Anim_BP.Launch Projectiles`
  (params (Projectile :type "/Game/Enums/Projectile_Type Enum" :default "NewEnumerator0"))
  (`self.Launch Proj` Projectile)
  (`ActorComponent.SetActive` (`self.Niagara`) false false)
  (`ActorComponent.SetActive` (`self.Niagara1`) false false))

(event `/Game/Platformer/Blueprints/Player/Animations/Player_Anim_BP.Charge Projectiles`
  (params (Projectile :type "/Game/Enums/Projectile_Type Enum" :default "NewEnumerator0"))
  (switch `/Game/Enums/Projectile_Type` Projectile
    (:`NewEnumerator0`
      (`ActorComponent.SetActive` (`self.Niagara1`) true false))
    (:`NewEnumerator1`
      (`ActorComponent.SetActive` (`self.Niagara`) true false))))

(event `KnockPlayer`
  (if (and (< (`KismetMathLibrary.Vector_Distance` (`self.K2_GetActorLocation` (`self.Player_ref`)) (`self.K2_GetActorLocation`)) (`self.Attack Distance`)) (not (`self.Dead`)) (`self.Can Knock`) (not (`/Game/Platformer/Blueprints/Player/Player_BP.Dead` (`self.Player_ref`))))
    (`/Engine/EditorBlueprintResources/StandardMacros.DoOnce` false :!label _label_4
      (:`Completed`
        (`NiagaraFunctionLibrary.SpawnSystemAtLocation` "/Game/Sci-Fi_Starter_VFX_Pack_Niagara/Niagara/Shield/NS_Shield_7.NS_Shield_7" (`SceneComponent.GetSocketLocation` (`self.Mesh`) "spine_03") (struct) (`self.GetActorScale3D`))
        (`/Game/Platformer/Blueprints/Player/Player_BP.KnockBack` (`self.Player_ref`) self (`self.Knockback Force`))
        (`KismetSystemLibrary.Delay` 20.0)
        (goto _label_4 :!via `Reset`)))))

(fn `Launch Proj`
  (params (Selection :type "/Game/Enums/Projectile_Type Enum" :default "NewEnumerator0"))
  (locals (Projectiles :type "/Game/Platformer/Blueprints/Projectiles/Projectile_BP Class Reference"))
  (bind (_returnvalue_location _returnvalue_rotation _returnvalue_scale) (`KismetMathLibrary.BreakTransform` (`self.GetTransform`)))
  (bind _shoot_speed (`self.Shoot Speed`))
  (bind _returnvalue (`SceneComponent.GetSocketLocation` (`self.StaticMesh`) "Top_socket"))
  (switch `/Game/Enums/Projectile_Type` Selection
    (:`NewEnumerator0`
      (set `local.Projectiles` "/Game/Platformer/Blueprints/Projectiles/FireBall_BP.FireBall_BP_C"))
    (:`NewEnumerator1`
      (set `local.Projectiles` "/Game/Platformer/Blueprints/Projectiles/BigFireBall_BP.BigFireBall_BP_C")))
  (bind _returnvalue_2 (`|SpawnActorFromClass` (`local.Projectiles`) (`KismetMathLibrary.MakeTransform` _returnvalue (`KismetMathLibrary.FindLookAtRotation` _returnvalue (`self.K2_GetActorLocation` (`self.Player_ref`))) _returnvalue_scale) "Undefined" "OverrideRootScale" null null))
  (`/Engine/EditorBlueprintResources/StandardMacros.IsValid` _returnvalue_2
    (:`Is Valid`
      (bind _projectilemovement (`/Game/Platformer/Blueprints/Projectiles/Projectile_BP.ProjectileMovement` _returnvalue_2))
      (set `ProjectileMovementComponent.MaxSpeed` _shoot_speed _projectilemovement)
      (set `ProjectileMovementComponent.InitialSpeed` _shoot_speed _projectilemovement))))

(fn `UserConstructionScript`
  (bind _returnvalue_x (`KismetMathLibrary.BreakVector` (`self.GetActorScale3D`)))
  (`SceneComponent.K2_AttachToComponent` (`self.StaticMesh`) (`self.Mesh`) "hand_rSocket" "SnapToTarget" "SnapToTarget" "SnapToTarget" true)
  (`SphereComponent.SetSphereRadius` (`self.Follow_trigger`) (/ (`self.Follow Distance`) _returnvalue_x) true)
  (`SphereComponent.SetSphereRadius` (`self.Attack_trigger`) (/ (`self.Attack Distance`) _returnvalue_x) true))