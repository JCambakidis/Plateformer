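; Pickup Blueprint for the platformer: a spinning item that the player collects by touching it.
; Tick rotates the mesh around yaw by a fixed step each frame, independent of delta time.
; When the player overlaps its box, it passes itself to the player's pickup feedback function, then destroys itself.
; The construction script traces downward and, on a hit, snaps the actor to hover a fixed height above the surface below.
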(event `self.ReceiveTick`
  (params (DeltaSeconds :type "Float (single-precision)"))
  (`SceneComponent.K2_AddWorldRotation` (`self.Mesh`) (struct :`Yaw` 3.0) false false))

(event `self.Box.OnComponentBeginOverlap`
  (params (OverlappedComponent :type "PrimitiveComponent Object Reference") (OtherActor :type "Actor Object Reference") (OtherComp :type "PrimitiveComponent Object Reference") (OtherBodyIndex :type Integer) (bFromSweep :type Boolean) (SweepResult :type "HitResult Structure (by ref)"))
  (bind _asplayer_bp (cast `/Game/Platformer/Blueprints/Player/Player_BP` OtherActor))
  (`/Game/Platformer/Blueprints/Player/Player_BP.Pickup_FeedBack` _asplayer_bp self)
  (`self.K2_DestroyActor`))

(fn `UserConstructionScript`
  (bind _returnvalue (`self.K2_GetActorLocation`))
  (bind (_outhit _returnvalue_2) (`KismetSystemLibrary.LineTraceSingle` _returnvalue (`KismetMathLibrary.MakeVector` (.x _returnvalue) (.y _returnvalue) (- (.z _returnvalue) 300.0)) "TraceTypeQuery1"))
  (if _returnvalue_2
    (`self.K2_SetActorLocation` (`KismetMathLibrary.MakeVector` (.x (`.ImpactPoint` (`GameplayStatics.BreakHitResult` _outhit))) (.y (`.ImpactPoint` (`GameplayStatics.BreakHitResult` _outhit))) (+ (.z (`.ImpactPoint` (`GameplayStatics.BreakHitResult` _outhit))) 100.0)))))