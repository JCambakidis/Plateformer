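; Platformer projectile that damages the player on contact and destroys itself after ten seconds if still alive.
; A sphere overlap with Player_BP spawns a Niagara explosion at half the actor's scale, applies knockback and damage, then destroys the projectile.
; Other overlaps spawn a smaller explosion, but their knockback and destroy require the failed cast's player reference, so the projectile persists.
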(event `self.ReceiveBeginPlay`
  (`KismetSystemLibrary.Delay` 10.0)
  (`self.K2_DestroyActor`))

(event `self.Sphere1.OnComponentBeginOverlap`
  (params (OverlappedComponent :type "PrimitiveComponent Object Reference") (OtherActor :type "Actor Object Reference") (OtherComp :type "PrimitiveComponent Object Reference") (OtherBodyIndex :type Integer) (bFromSweep :type Boolean) (SweepResult :type "HitResult Structure (by ref)"))
  (bind (_returnvalue_location _returnvalue_rotation _returnvalue_scale) (`KismetMathLibrary.BreakTransform` (`self.GetTransform`)))
  (bind _returnvalue (/ _returnvalue_scale 2))
  (bind _asplayer_bp (cast `/Game/Platformer/Blueprints/Player/Player_BP` OtherActor)
    (:`then`
      (`/Engine/EditorBlueprintResources/StandardMacros.IsValid` self
        (:`Is Valid`
          (`NiagaraFunctionLibrary.SpawnSystemAtLocation` "/Game/Sci-Fi_Starter_VFX_Pack_Niagara/Niagara/Explosion/NS_Explosion_C4_2.NS_Explosion_C4_2" (`self.K2_GetActorLocation`) (struct) _returnvalue)
          (`/Engine/EditorBlueprintResources/StandardMacros.IsValid` self
            (:`Is Valid`
              (`/Game/Platformer/Blueprints/Player/Player_BP.KnockBack` _asplayer_bp self 10.0)
              (`/Game/Platformer/Blueprints/Player/Player_BP.Take Damage` _asplayer_bp))))))
    (:`CastFailed`
      (`/Engine/EditorBlueprintResources/StandardMacros.IsValid` self
        (:`Is Valid`
          (`NiagaraFunctionLibrary.SpawnSystemAtLocation` "/Game/Sci-Fi_Starter_VFX_Pack_Niagara/Niagara/Explosion/NS_Explosion_Small_2.NS_Explosion_Small_2" (`self.K2_GetActorLocation`) (struct) _returnvalue)
          (`/Engine/EditorBlueprintResources/StandardMacros.IsValid` self
            (:`Is Valid`
              (`/Engine/EditorBlueprintResources/StandardMacros.IsValid` _asplayer_bp
                (:`Is Valid`
                  (`/Game/Platformer/Blueprints/Player/Player_BP.KnockBack` _asplayer_bp self 3.0)))))))))
  (`self.K2_DestroyActor`))

(fn `UserConstructionScript`)