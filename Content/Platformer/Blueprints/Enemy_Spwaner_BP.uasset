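; Enemy spawner actor for the Platformer game that repeatedly spawns Enemie_BP enemies at random points inside its box volume.
; The construction script sizes the box from BoxExtends.
; BeginPlay caches the first Player_BP and triggers the first spawn.
; Each successful spawn passes that player reference to the new enemy and sets a looping SpawnRate timer that calls SpawnEnemy again.
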(event `self.ReceiveBeginPlay`
  (bind _outactors (`GameplayStatics.GetAllActorsOfClass` "/Game/Platformer/Blueprints/Player/Player_BP.Player_BP_C"))
  (set `self.Player ref` (`|GetArrayItem` _outactors))
  (`self.Spawn enemy`))

(event `Spawn enemy`
  (bind _returnvalue (`|SpawnActorFromClass` "/Game/Platformer/Blueprints/Enemies/Enemie_BP.Enemie_BP_C" (`KismetMathLibrary.MakeTransform` (`KismetMathLibrary.RandomPointInBoundingBox` (`self.K2_GetActorLocation`) (`BoxComponent.BoxExtent` (`self.Box`)))) "Undefined" "OverrideRootScale" null null))
  (`/Engine/EditorBlueprintResources/StandardMacros.IsValid` _returnvalue
    (:`Is Valid`
      (set `/Game/Platformer/Blueprints/Enemies/Enemie_BP.Player_ref` (`self.Player ref`) _returnvalue)
      (`KismetSystemLibrary.K2_SetTimerDelegate` (delegate `Spawn enemy`) (`self.spawn rate`) true))))

(fn `UserConstructionScript`
  (`BoxComponent.SetBoxExtent` (`self.Box`) (`self.Box extends`) true))