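; Teleportation portal for the platformer that warps the player to a linked destination portal.
; When Player_BP overlaps the Box while CanWarp is true, it zeroes movement velocity, teleports the player to the destination's SpawnPoint and applies that point's rotation to the player's mesh.
; It disables the destination's CanWarp before the move and restores it after a short delay, preventing an immediate bounce back.
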(event `self.Box.OnComponentBeginOverlap`
  (params (OverlappedComponent :type "PrimitiveComponent Object Reference") (OtherActor :type "Actor Object Reference") (OtherComp :type "PrimitiveComponent Object Reference") (OtherBodyIndex :type Integer) (bFromSweep :type Boolean) (SweepResult :type "HitResult Structure (by ref)"))
  (bind _destination_portal (`self.Destination Portal`))
  (bind _spawn_point (`/Game/Platformer/Blueprints/Teleportation_Portal_BP.Spawn Point` _destination_portal))
  (bind (_returnvalue_roll _returnvalue_pitch _returnvalue_yaw) (`KismetMathLibrary.BreakRotator` (`SceneComponent.K2_GetComponentRotation` _spawn_point)))
  (if (`self.Can Warp`)
    (bind _asplayer_bp (cast `/Game/Platformer/Blueprints/Player/Player_BP` OtherActor))
    (set `/Game/Platformer/Blueprints/Teleportation_Portal_BP.Can Warp` false _destination_portal)
    (set `MovementComponent.Velocity` (0.0 0.0 0.0) (`Character.CharacterMovement` _asplayer_bp))
    (`self.K2_SetActorLocationAndRotation` :`self` _asplayer_bp :`NewLocation` (`SceneComponent.K2_GetComponentLocation` _spawn_point) :`bTeleport` true)
    (`SceneComponent.K2_SetWorldRotation` (`Character.Mesh` _asplayer_bp) (`KismetMathLibrary.MakeRotator` _returnvalue_roll _returnvalue_pitch _returnvalue_yaw) false false)
    (`KismetSystemLibrary.Delay` 0.5)
    (set `/Game/Platformer/Blueprints/Teleportation_Portal_BP.Can Warp` true _destination_portal)))

(fn `UserConstructionScript`)