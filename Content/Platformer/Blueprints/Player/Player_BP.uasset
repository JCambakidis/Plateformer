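; Player character for a platformer with sword combat, guarding, limited healing, coin pickups and knockback.
; Input drives movement, mesh-yaw turning and clamped camera pitch, while combat actions send messages to the AnimInstance.
; While CanAttack is set, Tick sphere-traces between sword sockets, damaging enemies absent from a hit list.
; It also creates the HUD, tracks lives and death, and restores position using registered falling points or the start location.
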(event `KnockBack`
  (params (Actor :type "Actor Object Reference") (`Knockback Force` :type "Float (double-precision)"))
  (bind (_returnvalue_x _returnvalue_y) (`KismetMathLibrary.BreakVector` (`self.K2_GetActorLocation` Actor)))
  (bind (_returnvalue_x_2 _returnvalue_y_2) (`KismetMathLibrary.BreakVector` (`self.K2_GetActorLocation`)))
  (`/Engine/EditorBlueprintResources/StandardMacros.IsValid` Actor
    (:`Is Valid`
      (`CharacterMovementComponent.AddImpulse` (`self.CharacterMovement`) (* (`KismetMathLibrary.ClampVectorSize` (`KismetMathLibrary.MakeVector` (* (- _returnvalue_x _returnvalue_x_2) -1.0) (* (- _returnvalue_y _returnvalue_y_2) -1.0) 100.0) -10.0 100.0) `Knockback Force`) true))))

(event `Pickup_FeedBack`
  (params (Pickup :type "Actor Object Reference"))
  ;[1 1 1] Pickup FeedBack
  (cast `/Game/Platformer/Blueprints/GamePlay_Elements/Coin_BP` Pickup)
  (`/Engine/EditorBlueprintResources/StandardMacros.IncrementInt` (`self.Coins Counter`)
    (:`  `
      (`NiagaraFunctionLibrary.SpawnSystemAtLocation` "/Game/Sci-Fi_Starter_VFX_Pack_Niagara/Niagara/Impact/NS_Impact_Mesh_Bounce.NS_Impact_Mesh_Bounce" (`self.K2_GetActorLocation`)))))

(event `Take Damage`
  (bind _returnvalue (`SkeletalMeshComponent.GetAnimInstance` (`self.Mesh`)))
  ;[1 1 1] Sub life if player is hit and no guard
  (if (and (not (`self.On Guard`)) (`self.Can Be Damage`))
    (`NiagaraFunctionLibrary.SpawnSystemAtLocation` "/Game/Sci-Fi_Starter_VFX_Pack_Niagara/Niagara/Blood/NS_Blood_Splat_3D_2.NS_Blood_Splat_3D_2" (`self.K2_GetActorLocation`) (struct) (2.0 2.0 2.0))
    (bind _result (`/Engine/EditorBlueprintResources/StandardMacros.DecrementInt` (`self.Life`))
      (:`  `
        (if (== _result 0)
          (message `/Game/Platformer/Blueprints/Player/Animations/Player_Anim_BP.Die` _returnvalue)
          (set `self.Dead` true)
          (set `PlayerController.bShowMouseCursor` true (`GameplayStatics.GetPlayerController` 0))
          (else
            (message `/Game/Platformer/Blueprints/Player/Animations/Player_Anim_BP.Hit` _returnvalue :!label _label)))))
    (else
      (goto _label))))

(event `self.ReceiveBeginPlay`
  ;[1 1 1] Begin Play
  (set `self.Init location` (`self.K2_GetActorLocation`))
  (bind _returnvalue (`|CreateWidget` "/Game/Platformer/Widgets/HUD_W.HUD_W_C" (`GameplayStatics.GetPlayerController` 0)))
  (set `self.HUD` _returnvalue)
  (set `/Game/Platformer/Widgets/HUD_W.Player_Ref` self _returnvalue)
  (`UserWidget.AddToViewport` _returnvalue 0))

(event `Restore location`
  ;[1 1 1] Restore location to nearest falling point
  (if (> (`KismetArrayLibrary.Array_Length` (`self.Falling Points`)) 0)
    (bind _output (`self.Find Closest Falling Point`))
    (`self.K2_SetActorLocation` (`SceneComponent.K2_GetComponentLocation` (`/Game/Platformer/Blueprints/Player/Falling_Point_BP.DefaultSceneRoot` _output)))
    (else
      (`self.K2_SetActorLocation` (`self.Init location`)))))

(event `self.ReceiveTick`
  (params (DeltaSeconds :type "Float (single-precision)"))
  (bind _sword (`self.Sword`))
  (bind _hitted_enemys (`self.Hitted Enemys`))
  ;[1 1 1] Event tick
  (`|ExecutionSequence`
    (:`then_0`
      (if (`self.Can Attack`)
        (bind _outhit (`KismetSystemLibrary.SphereTraceSingle` (`SceneComponent.GetSocketLocation` _sword "Hit_start") (`SceneComponent.GetSocketLocation` _sword "Hit_end") 20.0 "TraceTypeQuery1"))
        (bind (_bblockinghit _binitialoverlap _time _distance _location _impactpoint _normal _impactnormal _physmat _hitactor) (`GameplayStatics.BreakHitResult` _outhit))
        (bind _asenemie_bp (cast `/Game/Platformer/Blueprints/Enemies/Enemie_BP` _hitactor))
        (if (not (`KismetArrayLibrary.Array_Contains` _hitted_enemys _hitactor))
          (`/Game/Platformer/Blueprints/Enemies/Enemie_BP.Take Damage` _asenemie_bp)
          (`KismetArrayLibrary.Array_Add` _hitted_enemys _hitactor)
          (goto _label_2 :!via `Reset`))
        (else
          (`/Engine/EditorBlueprintResources/StandardMacros.DoOnce` true :!label _label_2
            (:`Completed`
              (`KismetArrayLibrary.Array_Clear` (`self.Hitted Enemys`)))))))))

(event `OnTakeAnyDamage_Event_0`
  (params (DamagedActor :type "Actor Object Reference") (Damage :type "Float (double-precision)") (DamageType :type "DamageType Object Reference") (InstigatedBy :type "Controller Object Reference") (DamageCauser :type "Actor Object Reference"))
  ;[1 1 1] Event tick
)

(event `Add FallingPoints`
  (params (`Falling Point` :type "/Game/Platformer/Blueprints/Player/Falling_Point_BP Object Reference"))
  ;[1 1 1] Add falling point to array
  (`KismetArrayLibrary.Array_Add` (`self.Falling Points`) `Falling Point`))

(event `InputAction|Attack`
  (params (Key :type "Key Structure"))
  ;[1 1 1] Inputs Actions
  (:`Pressed`
    (if (and (not (`self.Dead`)) (not (`self.On Guard`)) (not (`NavMovementComponent.IsFalling` (`self.CharacterMovement`))))
      (message `/Game/Platformer/Blueprints/Player/Animations/Player_Anim_BP.Attack` (`SkeletalMeshComponent.GetAnimInstance` (`self.Mesh`))))))

(event `InputAxis|MoveForwad`
  (params (AxisValue :type "Float (single-precision)"))
  (bind (_returnvalue_roll _returnvalue_pitch _returnvalue_yaw) (`KismetMathLibrary.BreakRotator` (`SceneComponent.K2_GetComponentRotation` (`self.Mesh`))))
  ;[1 1 1] Movement inputs
  ;;[1 1 1] Input Moving
  (if (not (`self.Dead`))
    (`self.AddMovementInput` (`KismetMathLibrary.GetForwardVector` (`KismetMathLibrary.MakeRotator` _returnvalue_roll _returnvalue_pitch (+ _returnvalue_yaw 90.0))) AxisValue)))

(event `InputAxis|MoveRight`
  (params (AxisValue :type "Float (single-precision)"))
  ;[1 1 1] Movement inputs
  ;;[1 1 1] Input Moving
  (if (not (`self.Dead`))
    (`self.AddMovementInput` (`KismetMathLibrary.GetForwardVector` (`SceneComponent.K2_GetComponentRotation` (`self.Mesh`))) AxisValue)))

(event `InputAction|Jump`
  (params (Key :type "Key Structure"))
  ;[1 1 1] Inputs Actions
  (:`Pressed`
    (if (and (not (`self.Dead`)) (not (`self.On Guard`)))
      (`self.Jump`))))

(event `InputAxis|MoveRotation`
  (params (AxisValue :type "Float (single-precision)"))
  ;[1 1 1] Movement inputs
  ;;[1 1 1] Input Rotation
  (if (not (`self.Dead`))
    (`SceneComponent.K2_AddWorldRotation` (`self.Mesh`) (`KismetMathLibrary.MakeRotator` 0.0 0.0 (* AxisValue (`self.Rotation Speed`))) false false)))

(event `InputAction|Guard`
  (params (Key :type "Key Structure"))
  (bind _charactermovement (`self.CharacterMovement`))
  (bind _returnvalue (`SkeletalMeshComponent.GetAnimInstance` (`self.Mesh`)))
  ;[1 1 1] Inputs Actions
  (:`Pressed`
    (if (and (not (`self.Dead`)) (not (`NavMovementComponent.IsFalling` (`self.CharacterMovement`))))
      (bind _output_get (set `self.On Guard` true))
      (message `/Game/Platformer/Blueprints/Player/Animations/Player_Anim_BP.Guard` _returnvalue _output_get)
      (set `CharacterMovementComponent.MaxWalkSpeed` 400.0 _charactermovement)))
  (:`Released`
    (bind _output_get_2 (set `self.On Guard` false))
    (message `/Game/Platformer/Blueprints/Player/Animations/Player_Anim_BP.Guard` _returnvalue _output_get_2)
    (set `CharacterMovementComponent.MaxWalkSpeed` 1000.0 _charactermovement)))

(event `InputAxisKey|MouseX`
  (params (AxisValue :type "Float (single-precision)"))
  ;[1 1 1] Movement inputs
  ;;[1 1 1] Input Rotation
  (if (not (`self.Dead`))
    (`SceneComponent.K2_AddWorldRotation` (`self.Mesh`) (`KismetMathLibrary.MakeRotator` 0.0 0.0 (* AxisValue (/ (`self.Rotation Speed`) 3.0))) false false)))

(event `InputAxisKey|MouseY`
  (params (AxisValue :type "Float (single-precision)"))
  (bind _camera (`self.Camera`))
  (bind (_relativerotation_roll _relativerotation_pitch) (`KismetMathLibrary.BreakRotator` (`SceneComponent.RelativeRotation` _camera)))
  ;[1 1 1] Movement inputs
  ;;[1 1 1] Input Rotation
  (if (and (or (> _relativerotation_pitch -10.0) (> AxisValue 0.0)) (or (< _relativerotation_pitch 30.0) (< AxisValue 0.0)) (!= AxisValue 0.0))
    (`SceneComponent.K2_AddRelativeRotation` _camera (`KismetMathLibrary.MakeRotator` 0.0 (* AxisValue (/ (`self.Rotation Speed`) 20.0))) false false)))

(event `InputAction|Heal`
  (params (Key :type "Key Structure"))
  (bind _number_of_heal (`self.Number of heal`))
  (:`Pressed`
    (if (and (`self.Can Heal`) (and (not (`self.Dead`)) (not (`self.On Guard`)) (not (`NavMovementComponent.IsFalling` (`self.CharacterMovement`)))) (> _number_of_heal 0) (< (`self.Life`) 5))
      (set `self.Can Be Damage` false)
      (set `self.Can Heal` false)
      (`/Engine/EditorBlueprintResources/StandardMacros.DecrementInt` _number_of_heal
        (:`  `
          (set `self.Life` 5)
          (message `/Game/Platformer/Blueprints/Player/Animations/Player_Anim_BP.Heal` (`SkeletalMeshComponent.GetAnimInstance` (`self.Mesh`)))
          (`NiagaraFunctionLibrary.SpawnSystemAttached` "/Game/Sci-Fi_Starter_VFX_Pack_Niagara/Niagara/Shield/NS_Shield_2.NS_Shield_2" (`self.Mesh`) "spine_03" (0.0 0.0 0.0) (struct) "SnapToTarget")
          (`|ExecutionSequence`
            (:`then_0`
              (`KismetSystemLibrary.Delay` 3.0)
              (set `self.Can Heal` true))
            (:`then_1`
              (`KismetSystemLibrary.Delay` 1.5)
              (set `self.Can Be Damage` true))))))))

(fn `Find Closest Falling Point`
  (returns (Output :type "/Game/Platformer/Blueprints/Player/Falling_Point_BP Object Reference"))
  (locals (`Closest Distance` :type "Float (double-precision)") (Index :type Integer))
  (bind _falling_points (`self.Falling Points`))
  (set `local.Closest Distance` (`KismetMathLibrary.Vector_Distance` (`self.Init location`) (`self.K2_GetActorLocation`)))
  (for (_array_element _array_index) _falling_points
    (bind _returnvalue (`KismetMathLibrary.Vector_Distance` (`self.K2_GetActorLocation` _array_element) (`self.K2_GetActorLocation`)))
    (if (< _returnvalue (`local.Closest Distance`))
      (set `local.Closest Distance` _returnvalue)
      (set `local.Index` _array_index)))
  (return (`|GetArrayItem` _falling_points (`local.Index`))))

(fn `UserConstructionScript`
  (`SceneComponent.K2_AttachToComponent` (`self.Sword`) (`self.Mesh`) "hand_rSocket" "SnapToTarget" "KeepRelative" "SnapToTarget" true)
  (`SceneComponent.K2_AttachToComponent` (`self.Shield`) (`self.Mesh`) "hand_lSocket" "SnapToTarget" "KeepRelative" "SnapToTarget" true))