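; Main menu environment generator that creates an endlessly scrolling backdrop of randomly scattered props.
; Four ground meshes move along X by Speed every tick, without delta-time scaling.
; On hitting EndBox, a segment teleports 1600 units along X from its predecessor, destroys its props and regenerates them.
; GenerateEnvironment, also run at construction, attaches random StaticMeshsArray meshes with random position, yaw and scale inside each segment's box.
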(event `self.ReceiveTick`
  (params (DeltaSeconds :type "Float (single-precision)"))
  (bind _speed (`self.Speed`))
  (`SceneComponent.K2_AddRelativeLocation` (`self.StaticMesh`) (`KismetMathLibrary.MakeVector` _speed) false false)
  (`SceneComponent.K2_AddRelativeLocation` (`self.StaticMesh1`) (`KismetMathLibrary.MakeVector` _speed) false false)
  (`SceneComponent.K2_AddRelativeLocation` (`self.StaticMesh10`) (`KismetMathLibrary.MakeVector` _speed) false false)
  (`SceneComponent.K2_AddRelativeLocation` (`self.StaticMesh15`) (`KismetMathLibrary.MakeVector` _speed) false false))

(event `self.End Box.OnComponentBeginOverlap`
  (params (OverlappedComponent :type "PrimitiveComponent Object Reference") (OtherActor :type "Actor Object Reference") (OtherComp :type "PrimitiveComponent Object Reference") (OtherBodyIndex :type Integer) (bFromSweep :type Boolean) (SweepResult :type "HitResult Structure (by ref)"))
  (bind _staticmesh1 (`self.StaticMesh1`))
  (bind _staticmesh15 (`self.StaticMesh15`))
  (bind _elements1 (`self.Elements1`))
  (bind _elements2 (`self.Elements2`))
  (bind _elements3 (`self.Elements3`))
  (bind _elements4 (`self.Elements4`))
  (bind _staticmesh (`self.StaticMesh`))
  (bind _staticmesh10 (`self.StaticMesh10`))
  (bind _relativelocation_x (`KismetMathLibrary.BreakVector` (`SceneComponent.RelativeLocation` (`self.StaticMesh15`))))
  (bind _relativelocation_x_2 (`KismetMathLibrary.BreakVector` (`SceneComponent.RelativeLocation` (`self.StaticMesh10`))))
  (bind _relativelocation_x_3 (`KismetMathLibrary.BreakVector` (`SceneComponent.RelativeLocation` (`self.StaticMesh`))))
  (bind _relativelocation_x_4 (`KismetMathLibrary.BreakVector` (`SceneComponent.RelativeLocation` (`self.StaticMesh1`))))
  (if (== OtherComp _staticmesh)
    (`SceneComponent.K2_SetRelativeLocation` _staticmesh (`KismetMathLibrary.MakeVector` (+ _relativelocation_x 1600.0)) false true)
    (for _array_element _elements1
      (`ActorComponent.K2_DestroyComponent` _array_element))
    (`KismetArrayLibrary.Array_Clear` _elements1)
    (`self.Generate environment` (`self.Elements1`) (`self.StaticMesh`) (`self.Box`) 3 5 1 3)
    (elif (== OtherComp _staticmesh1)
      (`SceneComponent.K2_SetRelativeLocation` _staticmesh1 (`KismetMathLibrary.MakeVector` (+ _relativelocation_x_3 1600.0)) false true)
      (for _array_element_2 _elements2
        (`ActorComponent.K2_DestroyComponent` _array_element_2))
      (`KismetArrayLibrary.Array_Clear` _elements2)
      (`self.Generate environment` (`self.Elements2`) (`self.StaticMesh1`) (`self.Box1`) 3 5 1 3)
      (elif (== OtherComp _staticmesh10)
        (`SceneComponent.K2_SetRelativeLocation` _staticmesh10 (`KismetMathLibrary.MakeVector` (+ _relativelocation_x_4 1600.0)) false true)
        (for _array_element_3 _elements3
          (`ActorComponent.K2_DestroyComponent` _array_element_3))
        (`KismetArrayLibrary.Array_Clear` _elements3)
        (`self.Generate environment` (`self.Elements3`) (`self.StaticMesh10`) (`self.Box2`) 3 5 1 3)
        (elif (== OtherComp _staticmesh15)
          (`SceneComponent.K2_SetRelativeLocation` _staticmesh15 (`KismetMathLibrary.MakeVector` (+ _relativelocation_x_2 1600.0)) false true)
          (for _array_element_4 _elements4
            (`ActorComponent.K2_DestroyComponent` _array_element_4))
          (`KismetArrayLibrary.Array_Clear` _elements4)
          (`self.Generate environment` (`self.Elements4`) (`self.StaticMesh15`) (`self.Box3`) 3 5 1 3))))))

(fn `Add Environment Elements`
  (params (`Number Of elements` :type Integer) (`Save Tab` :type "Array of StaticMeshComponent Object Reference") (`Spawn Box` :type "BoxComponent Object Reference") (Mesh :type "StaticMesh Object Reference") (`Parent Mesh` :type "SceneComponent Object Reference"))
  (bind (_returnvalue_x _returnvalue_y _returnvalue_z) (`KismetMathLibrary.BreakVector` (`self.K2_GetActorLocation`)))
  (bind _returnvalue (`KismetMathLibrary.RandomFloatInRange` 0.5 2.0))
  (bind (_returnvalue_x_2 _returnvalue_y_2) (`KismetMathLibrary.BreakVector` (`KismetMathLibrary.RandomPointInBoundingBox` (`SceneComponent.K2_GetComponentLocation` `Spawn Box`) (`BoxComponent.BoxExtent` `Spawn Box`))))
  (for _ (range (+ `Number Of elements` 1))
    (bind _returnvalue_2 (`AddComponent|NODE_AddStaticMeshComponent-0` :`bManualAttachment` true :`RelativeTransform` (`KismetMathLibrary.MakeTransform` (`KismetMathLibrary.MakeVector` _returnvalue_x_2 _returnvalue_y_2 _returnvalue_z) (`KismetMathLibrary.MakeRotator` 0.0 0.0 (`KismetMathLibrary.RandomFloatInRange` -90.0 90.0)) (`KismetMathLibrary.MakeVector` _returnvalue _returnvalue _returnvalue))))
    (`SceneComponent.K2_AttachToComponent` _returnvalue_2 `Parent Mesh` "None" "KeepWorld" "KeepRelative" "KeepRelative" true)
    (`StaticMeshComponent.SetStaticMesh` _returnvalue_2 Mesh)
    (`KismetArrayLibrary.Array_Add` `Save Tab` _returnvalue_2)))

(fn `UserConstructionScript`
  (`self.Generate environment` (`self.Elements1`) (`self.StaticMesh`) (`self.Box`) 3 5 1 3)
  (`self.Generate environment` (`self.Elements2`) (`self.StaticMesh1`) (`self.Box1`) 3 5 1 3)
  (`self.Generate environment` (`self.Elements3`) (`self.StaticMesh10`) (`self.Box2`) 3 5 1 3)
  (`self.Generate environment` (`self.Elements4`) (`self.StaticMesh15`) (`self.Box3`) 3 5 1 3))